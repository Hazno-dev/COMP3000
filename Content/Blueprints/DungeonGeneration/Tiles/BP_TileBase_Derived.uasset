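; Dungeon generation tile Blueprint that gives designers a visual interface for setting which directions a tile connects.
; Its construction script loops over the TileConnections map and shows or hides the North, East, South and West components to match each value, both in editor and in game.
; Components are picked by loop index rather than key, so the mapping depends on map order.
; The event graph holds no active logic.
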(fn `UserConstructionScript`
  (bind _tileconnections (`self.TileConnections`))
  ;[1 1 1] Visual Interface for designing tile directions
  (bind _keys (`BlueprintMapLibrary.Map_Keys` _tileconnections))
  (for (_array_element _array_index) _keys
    (bind _value (`BlueprintMapLibrary.Map_Find` _tileconnections _array_element))
    (if _value
      _
      (else
        _))
    (bind _returnvalue (select `int` _array_index :`0` (`self.North`) :`1` (`self.East`) :`2` (`self.South`) :`3` (`self.West`)))
    (`SceneComponent.SetVisibility` _returnvalue _value false)
    (`SceneComponent.SetHiddenInGame` _returnvalue (not _value) false)))